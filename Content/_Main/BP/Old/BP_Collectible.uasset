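; A crystal collectible for the puzzle game that the player picks up by touching it.
; On BeginPlay it caches the puzzle game mode and adds a rotating movement component so it spins.
; When the player character overlaps it, it reports the pickup to the game mode's crystal counter and destroys itself.
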(event `self.ReceiveBeginPlay`
  ;[1 1 1] Initialize Collectible
  (bind _asbp_game_mode_puzzle_game (cast `/Game/_Main/BP/BP_GameMode_PuzzleGame` (`GameplayStatics.GetGameMode`)))
  (set `self.My Game Mode` _asbp_game_mode_puzzle_game)
  (`self.Initialize`))

(event `self.ReceiveActorBeginOverlap`
  (params (OtherActor :type "Actor Object Reference"))
  ;[1 1 1] Check if player collides
  (if (== OtherActor (`GameplayStatics.GetPlayerCharacter` 0))
    ;[1 1 1] PickUp to counter and destroy
    (`/Game/_Main/BP/BP_GameMode_PuzzleGame.CrystalPickup` (`self.My Game Mode`))
    (`self.K2_DestroyActor`)))

(fn `Initialize`
  (`AddComponent|NODE_AddRotatingMovementComponent-1`))

(fn `UserConstructionScript`)