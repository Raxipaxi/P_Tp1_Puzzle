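; Movable trap actor that damages the player character on overlap by sending it a TakeDamageMessage.
; Tick runs through a one-second Delay and a Seconds countdown, alternating between a 200-unit swept teleport upward and a reset.
; The reset uses a hardcoded world position rather than the placed location, and BeginPlay only re-sets the actor's current location.
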(event `self.ReceiveActorBeginOverlap`
  (params (OtherActor :type "Actor Object Reference"))
  (bind _returnvalue (`GameplayStatics.GetPlayerCharacter` 0))
  (if (== OtherActor _returnvalue)
    (message `/Game/_Main/BP/BPI_Damageable.TakeDamage` _returnvalue (`self.Damage`))))

(event `self.ReceiveBeginPlay`
  ;[1 0.4431 0.513] Move Trap
  (`self.K2_SetActorLocation` (`self.K2_GetActorLocation`)))

(event `Move Up`
  ;[1 0.4431 0.513] Move Trap
  (`self.K2_SetActorLocation` (+ (`self.K2_GetActorLocation`) (0.0 0.0 200.0)) true true))

(event `Reset Position`
  ;[1 0.4431 0.513] Move Trap
  (`self.K2_SetActorLocation` (-1470.0 50.0 -280.0) true true))

(event `self.ReceiveTick`
  (params (DeltaSeconds :type "Float (single-precision)"))
  ;[0.6342 1 0.8782] Timer
  (`KismetSystemLibrary.Delay` 1.0)
  (if (== (`self.Seconds`) 0.0)
    (set `self.Seconds` 1.0)
    (`self.Reset Position`)
    (else
      (set `self.Seconds` (- (`self.Seconds`) 1.0))
      (`self.Move Up`))))

(fn `UserConstructionScript`)