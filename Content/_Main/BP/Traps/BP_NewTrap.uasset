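; Trap actor that damages the player on contact and moves its mesh along the Z axis.
; Overlap on the trap mesh sends the Damage value to player character 0 through TakeDamageMessage, ignoring other actors.
; A timeline started at BeginPlay lerps the mesh's relative location, without sweep, between the cached actor world location and a small upward offset from it.
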(event `self.SM_NewTrap.OnComponentBeginOverlap`
  (params (OverlappedComponent :type "PrimitiveComponent Object Reference") (OtherActor :type "Actor Object Reference") (OtherComp :type "PrimitiveComponent Object Reference") (OtherBodyIndex :type Integer) (bFromSweep :type Boolean) (SweepResult :type "HitResult Structure (by ref)"))
  (bind _returnvalue (`GameplayStatics.GetPlayerCharacter` 0))
  (if (== OtherActor _returnvalue)
    (message `/Game/_Main/BP/BPI_Damageable.TakeDamage` _returnvalue (`self.Damage`))))

(event `self.ReceiveBeginPlay`
  ;[1 0.4431 0.513] Move Trap
  (bind _output_get (set `self.BaseLocation` (`self.K2_GetActorLocation`)))
  (bind (_direction _traptimetrack) (`Timeline|Timeline_0`)
    (:`Update`
      (`SceneComponent.K2_SetRelativeLocation` (`self.SM_NewTrap`) (`KismetMathLibrary.VLerp` _output_get (+ _output_get (0.0 0.0 10.0)) _traptimetrack) false false))))

(fn `UserConstructionScript`)