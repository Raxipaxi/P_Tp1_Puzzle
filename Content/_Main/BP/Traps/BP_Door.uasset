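; BP_Door is a trap door actor that moves between two heights and damages the player on overlap.
; When player character 0 begins overlapping it, it prints a debug string and sends that character a TakeDamage message with its Damage value.
; Every Tick it snaps, without sweep or interpolation, to a hardcoded world location, lower while PlayerIsOnTop is true.
; Nothing in these graphs sets PlayerIsOnTop.
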(event `self.ReceiveActorBeginOverlap`
  (params (OtherActor :type "Actor Object Reference"))
  (bind _returnvalue (`GameplayStatics.GetPlayerCharacter` 0))
  ;[1 0.5639 0.9262] Do Damage To Player
  (if (== OtherActor _returnvalue)
    (`KismetSystemLibrary.PrintString` "Player is here!")
    (message `/Game/_Main/BP/BPI_Damageable.TakeDamage` _returnvalue (`self.Damage`))))

(event `self.ReceiveTick`
  (params (DeltaSeconds :type "Float (single-precision)"))
  ;[0.2067 1 0.6933] Door movement
  (if (`self.PlayerIsOnTop`)
    (`self.K2_SetActorLocation` (480.0 35.0 -280.0))
    (else
      (`self.K2_SetActorLocation` (480.0 35.0 -110.0)))))

(fn `UserConstructionScript`)