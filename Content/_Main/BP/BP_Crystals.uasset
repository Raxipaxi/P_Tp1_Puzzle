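; BP_Crystals is a crystal actor that flies into the player when touched, then disappears.
; An overlap with the first player's pawn stores the crystal's current location and plays a timeline.
; Each update lerps the actor from that start point to the pawn's live position, so it homes in on a moving player.
; The actor destroys itself when the timeline finishes, with no reward logic in this graph.
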(event `self.ReceiveActorBeginOverlap`
  (params (OtherActor :type "Actor Object Reference"))
  (if (== OtherActor (`GameplayStatics.GetPlayerPawn` 0))
    (set `self.LerpSartLocation` (`self.K2_GetActorLocation`))
    (bind (_direction _smoothlerp) (`Timeline|Timeline_0`)
      (:`Update`
        (`self.K2_SetActorLocation` (`KismetMathLibrary.VLerp` (`self.LerpSartLocation`) (`self.K2_GetActorLocation` (`GameplayStatics.GetPlayerPawn` 0)) _smoothlerp)))
      (:`Finished`
        (`self.K2_DestroyActor`)))))

(fn `UserConstructionScript`)