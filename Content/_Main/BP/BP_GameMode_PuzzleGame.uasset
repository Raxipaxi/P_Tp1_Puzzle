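; Game mode for a puzzle game that tracks the countdown, tries, collectable count and game-over state.
; On BeginPlay it resets that state, starts a looping one-second Clock timer and streams in levels C1 and H1.
; Each tick runs macros that decrement time and check tries, ending the game and clearing the timer when either reaches zero.
; CrystalPickup adds a collectable and bonus time, while CoinLose removes a collectable.
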(event `self.ReceiveBeginPlay`
  ;[0 1 0.4646] Start Level
  (`self.StartGame`
    (:`Out`
      (`GameplayStatics.LoadStreamLevel` "C1" true)
      (`GameplayStatics.LoadStreamLevel` "H1" true))))

(event `Clock`
  ;[0 0.2636 1] Timer
  (`self.CheckTime`
    (:`NoTimeLeft`
      _)
    (:`TimeKeeps`
      (`self.CheckTries`
        (:`NoMoreTries`
          _))))
  (set `self.GameOver` true)
  (`KismetSystemLibrary.K2_ClearTimer` null "Clock"))

(fn `Coin Lose`
  (set `self.CollectableCount` (- (`self.CollectableCount`) 1)))

(fn `CrystalPickup`
  ;[1 1 1] Crystal Pickup
  (set `self.CollectableCount` (+ (`self.CollectableCount`) 1))
  (set `self.Time` (+ (`self.Time`) 5)))

(fn `NewFunction_0`)

(fn `UserConstructionScript`)