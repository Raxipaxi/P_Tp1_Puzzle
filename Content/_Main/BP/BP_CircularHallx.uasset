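; BP_CircularHallx is a circular hall actor whose base mesh rotates in two separately triggered stages.
; FirstRoll and SecondRoll each play their own timeline, turning the mesh in yaw toward a fixed angle, relative for the first and world for the second.
; Each update lerps from the current yaw rather than a stored start, so the motion is not a linear blend of timeline progress.
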(event `First Roll`
  (bind (_relativerotation_roll _relativerotation_pitch _relativerotation_yaw) (`KismetMathLibrary.BreakRotator` (`SceneComponent.RelativeRotation` (`self.SM_CircularHallBase`))))
  ;[1 1 1] First Rotation
  (bind (_direction _rotation_progress) (`Timeline|RotationTime`)
    (:`Update`
      (`SceneComponent.K2_SetRelativeRotation` (`self.SM_CircularHallBase`) (`KismetMathLibrary.MakeRotator` 0.0 0.0 (`KismetMathLibrary.Lerp` _relativerotation_yaw 5.0 _rotation_progress)) false false))))

(event `SecondRoll`
  (bind (_returnvalue_roll _returnvalue_pitch _returnvalue_yaw) (`KismetMathLibrary.BreakRotator` (`SceneComponent.K2_GetComponentRotation` (`self.SM_CircularHallBase`))))
  ;[1 1 1] Second Rotation
  (bind (_direction _rotation_progress) (`Timeline|Rotation Time 2`)
    (:`Update`
      (`SceneComponent.K2_SetWorldRotation` (`self.SM_CircularHallBase`) (`KismetMathLibrary.MakeRotator` 0.0 0.0 (`KismetMathLibrary.Lerp` _returnvalue_yaw 20.0 _rotation_progress)) false false))))

(fn `UserConstructionScript`)