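; BP_SwitchDoor is an overlap switch that sets the PlayerIsOnTop flag on a BP_Door.
; Begin overlap sets the flag when the overlapping actor is the player character or the first BP_Box found in the level.
; End overlap clears it only for the player, so a box leaving does not reset it.
; The target is the first BP_Door returned by GetAllActorsOfClass, with no per-switch reference.
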(event `self.ReceiveActorBeginOverlap`
  (params (OtherActor :type "Actor Object Reference"))
  ;[1 0.5501 0.59] Check overlapped actors
  (bind _outactors (`GameplayStatics.GetAllActorsOfClass` "/Game/_Main/BP/BP_Box.BP_Box_C"))
  (if (or (== (`|GetArrayItem` _outactors) OtherActor) (== OtherActor (`GameplayStatics.GetPlayerCharacter` 0)))
    (bind _outactors_2 (`GameplayStatics.GetAllActorsOfClass` "/Game/_Main/BP/Traps/BP_Door.BP_Door_C"))
    (set `/Game/_Main/BP/Traps/BP_Door.PlayerIsOnTop` true (`|GetArrayItem` _outactors_2))))

(event `self.ReceiveActorEndOverlap`
  (params (OtherActor :type "Actor Object Reference"))
  ;[1 0.5501 0.59] Check overlapped actors
  (if (== (`GameplayStatics.GetPlayerCharacter` 0) OtherActor)
    (bind _outactors (`GameplayStatics.GetAllActorsOfClass` "/Game/_Main/BP/Traps/BP_Door.BP_Door_C"))
    (set `/Game/_Main/BP/Traps/BP_Door.PlayerIsOnTop` false (`|GetArrayItem` _outactors))))

(fn `UserConstructionScript`)