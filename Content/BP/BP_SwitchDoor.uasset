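; BP_SwitchDoor is an overlap-triggered switch that opens and closes a BP_Door.
; Begin overlap calls OpenDoor when the other actor is the player character or the first BP_Box found.
; End overlap calls CloseDoor only for the player, whether or not the box still overlaps.
; Box and door are looked up with GetAllActorsOfClass at index 0, so only the first of each is used.
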(event `self.ReceiveActorBeginOverlap`
  (params (OtherActor :type "Actor Object Reference"))
  ;[1 0.5501 0.59] Check overlapped actors
  (bind _outactors (`GameplayStatics.GetAllActorsOfClass` "/Game/BP/BP_Box.BP_Box_C"))
  (if (or (== (`|GetArrayItem` _outactors) OtherActor) (== OtherActor (`GameplayStatics.GetPlayerCharacter` 0)))
    (bind _outactors_2 (`GameplayStatics.GetAllActorsOfClass` "/Game/BP/BP_Door.BP_Door_C"))
    (`/Game/BP/BP_Door.Open Door` (`|GetArrayItem` _outactors_2))))

(event `self.ReceiveActorEndOverlap`
  (params (OtherActor :type "Actor Object Reference"))
  ;[1 0.5501 0.59] Check overlapped actors
  (if (== (`GameplayStatics.GetPlayerCharacter` 0) OtherActor)
    (bind _outactors (`GameplayStatics.GetAllActorsOfClass` "/Game/BP/BP_Door.BP_Door_C"))
    (`/Game/BP/BP_Door.Close Door` (`|GetArrayItem` _outactors))))

(fn `UserConstructionScript`)