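; BP_Cannon is a cannon actor that fires automatically in an endless loop from BeginPlay.
; Each cycle waits for FireRate, reads the Arrow component's world location and rotation, then plays the CannonFire timeline, whose Recoil track moves the barrel along its relative Y axis.
; When the timeline finishes, it spawns a BP_Projectile at the captured transform, scaled by ProjectileScale, and loops back to the delay.
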(event `self.ReceiveBeginPlay`
  (`KismetSystemLibrary.Delay` (`self.FireRate`) :!label _label)
  (bind (_spawnlocation _spawnrotation) (`self.ArrowStartValues`))
  (bind (_direction _recoil) (`Timeline|CannonFire` :!via `PlayFromStart`)
    (:`Update`
      (`self.BarrelMovement` _recoil))
    (:`Finished`
      (`self.ProjectileSpawner` _spawnlocation _spawnrotation)
      (goto _label))))

(fn `ArrowStartValues`
  (returns (SpawnLocation :type "Vector Structure") (SpawnRotation :type "Rotator Structure"))
  (bind _arrow (`self.Arrow`))
  (return (`SceneComponent.K2_GetComponentLocation` _arrow) (`SceneComponent.K2_GetComponentRotation` _arrow)))

(fn `BarrelMovement`
  (params (NewLocation_Y :type "Float (double-precision)"))
  (`SceneComponent.K2_SetRelativeLocation` (`self.CannonBarrel`) (`KismetMathLibrary.MakeVector` 0.0 NewLocation_Y) false false))

(fn `ProjectileSpawner`
  (params (SpawnTransform_Location :type "Vector Structure") (SpawnTransform_Rotation :type "Rotator Structure"))
  (`|SpawnActorFromClass` "/Game/BluePrints/Actors/Projectile/BP_Projectile.BP_Projectile_C" (`KismetMathLibrary.MakeTransform` SpawnTransform_Location SpawnTransform_Rotation (`KismetMathLibrary.Conv_DoubleToVector` (`self.ProjectileScale`))) "Undefined" "OverrideRootScale" null null))

(fn `UserConstructionScript`)